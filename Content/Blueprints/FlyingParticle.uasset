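; Flying particle actor that loops along a referenced SplineBP spline once its create event fires, until the destroy event deactivates it.
; Tick matches the spline's location and rotation, advancing distance by a per-frame speed without delta time and wrapping to start.
; Self-rescheduling timers optionally alternate between two particle components for color changes and toggle speed boosts.
; The boost timer only starts when color change is also enabled.
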(event `self.ReceiveBeginPlay`
  (`ActorComponent.SetActive` (`self.Particle`) false true)
  (`ActorComponent.SetActive` (`self.ParticleSecondColor`) false true))

(event `Create the particles`
  (set `self.Active` true)
  (`ActorComponent.SetActive` (`self.Particle`) true true)
  (set `self.Distance Along Spline` 0.0)
  (`ActorComponent.SetActive` (`self.ParticleSecondColor`) false false)
  (if (`self.Change Color`)
    (`KismetSystemLibrary.K2_SetTimer` null "ChangeColor" (`self.Color Change start time`))
    (if (`self.IncreaseTravelSpeed`)
      (`KismetSystemLibrary.K2_SetTimer` null "IncreaseSpeed" (`self.Increment start time`)))))

(event `Destroy particles`
  (`ActorComponent.SetActive` (`self.Particle`) false true)
  (`ActorComponent.SetActive` (`self.ParticleSecondColor`) false true)
  (set `self.Active` false))

(event `self.ReceiveTick`
  (params (DeltaSeconds :type "Float (single-precision)"))
  (bind _travelspeed (`self.TravelSpeed`))
  (bind _distance_along_spline (`self.Distance Along Spline`))
  (bind _spline (`/Game/Blueprints/Spline.Spline` (`self.SplineBP`)))
  (bind _returnvalue (+ (`self.Distance Along Spline`) (`KismetMathLibrary.SelectFloat` (+ _travelspeed (`self.Speed Increment`)) _travelspeed (`self.IncreasedSpeed`))))
  (if (`self.Active`)
    (`|ExecutionSequence`
      (:`then_0`
        (`SceneComponent.K2_SetWorldRotation` (`SplineComponent.GetWorldRotationAtDistanceAlongSpline` _spline _distance_along_spline)))
      (:`then_1`
        (`SceneComponent.K2_SetWorldLocation` (`SplineComponent.GetWorldLocationAtDistanceAlongSpline` _spline _distance_along_spline)))
      (:`then_2`
        (set `self.Distance Along Spline` (`KismetMathLibrary.SelectFloat` 0.0 _returnvalue (>= _returnvalue (`SplineComponent.GetDistanceAlongSplineAtSplinePoint` _spline (- (`SplineComponent.GetNumSplinePoints` _spline) 1)))))))))

(fn `ChangeColor`
  (if (`self.Active`)
    (if (`self.Color Changed`)
      (`ActorComponent.SetActive` (`self.ParticleSecondColor`) false true)
      (`ActorComponent.SetActive` (`self.Particle`) true true)
      (set `self.Color Changed` false)
      (`KismetSystemLibrary.K2_SetTimer` null "ChangeColor" (`self.Color Change start time`))
      (else
        (`ActorComponent.SetActive` (`self.ParticleSecondColor`) true true)
        (`ActorComponent.SetActive` (`self.Particle`) false true)
        (set `self.Color Changed` true)
        (`KismetSystemLibrary.K2_SetTimer` null "ChangeColor" (`self.Color Change duration`))))))

(fn `IncreaseSpeed`
  (if (`self.IncreasedSpeed`)
    (set `self.IncreasedSpeed` false)
    (`KismetSystemLibrary.K2_SetTimer` null "IncreaseSpeed" (`self.Increment start time`))
    (else
      (set `self.IncreasedSpeed` true)
      (`KismetSystemLibrary.K2_SetTimer` null "IncreaseSpeed" (`self.Increment duration`)))))

(fn `UserConstructionScript`
  (`ActorComponent.SetActive` (`self.ParticleSecondColor`) false false))