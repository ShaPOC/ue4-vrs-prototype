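; BoostArrow is a speed-boost pickup actor that boosts the Avatar when overlapped while active.
; On overlap it deactivates itself, calls PlayerOverlap and then applies a fixed boost through the Avatar's BoostSpeed.
; SetActive stores the Active state and swaps the material between visible arrows and an invisible one, applied on BeginPlay from the initial value.
; Nothing in this Blueprint reactivates the arrow after use.
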(event `self.ReceiveBeginPlay`
  (`self.SetActive` (`self.Active`)))

(event `self.ReceiveActorBeginOverlap`
  (params (OtherActor :type "Actor Object Reference"))
  (if (and (== (`GameplayStatics.GetObjectClass` OtherActor) "/Game/Blueprints/Avatar.Avatar_C") (`self.Active`))
    (`self.SetActive` false)
    (`self.PlayerOverlap`)
    (bind _asavatar (cast `/Game/Blueprints/Avatar` OtherActor))
    (`/Game/Blueprints/Avatar.Boost Speed` _asavatar 5000.0)))

(event `self.ReceiveTick`
  (params (DeltaSeconds :type "Float (single-precision)")))

(fn `SetActive`
  (params (Active :type Boolean :default false))
  ;[1 1 1] Toggle and branch
  (`|ExecutionSequence`
    (:`then_0`
      (if Active
        (if (not (== (`PrimitiveComponent.GetMaterial` 0) "/Game/Materials/SpeedUpArrows.SpeedUpArrows"))
          (`PrimitiveComponent.SetMaterial` 0 "/Game/Materials/SpeedUpArrows.SpeedUpArrows"))
        (else
          (`PrimitiveComponent.SetMaterial` 0 "/Game/Materials/ArrowInvisible.ArrowInvisible"))))
    (:`then_1`
      (set `self.Active` Active))))

(fn `UserConstructionScript`)