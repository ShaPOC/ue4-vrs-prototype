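; FadeWall is a Blueprint with a static mesh that fades between transparent and opaque using the FadeOutBlack material.
; On BeginPlay it applies a dynamic instance of that material and sets its starting Opacity from the Active flag.
; The FadeNow event plays the Fade timeline to drive Opacity, with its In argument choosing between fading in and fading out.
; The timeline uses Play rather than PlayFromStart, so it never rewinds between calls.
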(event `self.ReceiveBeginPlay`
  (bind _returnvalue (`KismetMaterialLibrary.CreateDynamicMaterialInstance` "/Game/Effects/FadeOutBlack.FadeOutBlack"))
  (bind _output_get (set `self.Mat` _returnvalue))
  (`PrimitiveComponent.SetMaterial` (`self.StaticMesh`) 0 _output_get)
  (`MaterialInstanceDynamic.SetScalarParameterValue` _output_get "Opacity" (`KismetMathLibrary.SelectFloat` 1.0 0.0 (`self.Active`))))

(event `FadeNow`
  (params (In :type Boolean))
  (bind (_direction _fadefloat) (`Timeline|Fade`)
    (:`Update`
      (`MaterialInstanceDynamic.SetScalarParameterValue` (`self.Mat`) "Opacity" (`KismetMathLibrary.SelectFloat` (`KismetMathLibrary.Lerp` 0.0 1.0 _fadefloat) (`KismetMathLibrary.Lerp` 1.0 0.0 _fadefloat) In)))))

(event `self.ReceiveActorBeginOverlap`
  (params (OtherActor :type "Actor Object Reference")))

(event `self.ReceiveTick`
  (params (DeltaSeconds :type "Float (single-precision)")))

(fn `UserConstructionScript`)